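; BP_SmokeProjectile is a timed projectile that explodes one second after it begins play.
; On explosion it spawns a smoke emitter and applies radial damage at its location, credited to the instigator's controller.
; It also draws a debug sphere showing the damage radius, then destroys itself.
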(event `self.ReceiveBeginPlay`
  (`KismetSystemLibrary.Delay` 1.0)
  (`self.Explode`))

(event `Explode`
  (bind _returnvalue (`self.K2_GetActorLocation`))
  (`GameplayStatics.SpawnEmitterAtLocation` "/Game/PolygonHeist/ParticleFX/FX_Smoke.FX_Smoke" _returnvalue)
  (`GameplayStatics.ApplyRadialDamage` :`BaseDamage` (`self.Damage`) :`Origin` _returnvalue :`DamageRadius` (`self.DamageRadius`) :`DamageCauser` self :`InstigatedByController` (`self.GetInstigatorController`))
  (`KismetSystemLibrary.DrawDebugSphere` _returnvalue (`self.DamageRadius`) 12 (struct :`R` 1.0 :`G` 1.0 :`B` 1.0 :`A` 1.0) 1.0 1.0)
  (`self.K2_DestroyActor`))

(fn `UserConstructionScript`)